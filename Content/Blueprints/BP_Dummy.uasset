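; BP_Dummy is a damageable test dummy that shows its HUD and floating damage numbers when hit.
; On BeginPlay it caches the Health stat from its StatContainer, then sets base health through a stat modifier.
; AnyDamage reveals the HUD if hidden and spawns popup text of the damage amount at the Arrow's location.
; The graphs shown do not subtract damage from Health.
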(event `self.ReceiveBeginPlay`
  (`|ExecutionSequence`
    (:`then_0`
      (bind _returnvalue (`StatContainer.GetStat` (`self.StatContainer`) "Health"))
      (bind _ashealth_stat (cast `HealthStat` _returnvalue))
      (set `self.Health Stat` _ashealth_stat))
    (:`then_1`
      (`StatContainer.AddModifier` (`self.StatContainer`) (make `StatModifier` "Health" "Base" 100.0)))))

(event `self.ReceiveAnyDamage`
  (params (Damage :type "Float (single-precision)") (DamageType :type "DamageType Object Reference") (InstigatedBy :type "Controller Object Reference") (DamageCauser :type "Actor Object Reference"))
  (`|ExecutionSequence`
    (:`then_0`
      (if (not (`SceneComponent.IsVisible` (`self.HUD`)))
        (`SceneComponent.SetVisibility` (`self.HUD`) true false)))
    (:`then_1`
      (`/Game/Blueprints/Macros/PopupMacro.PopupTextSpawn` "/Game/Blueprints/PopupText/Blueprints/BP_DamagePopup.BP_DamagePopup_C" (`SceneComponent.K2_GetComponentLocation` (`self.Arrow`)) (`KismetTextLibrary.Conv_DoubleToText` Damage "HalfToEven")))))

(fn `UserConstructionScript`)