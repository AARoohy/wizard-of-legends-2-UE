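; Fire Arcana ability that fires a three-step fireball combo, advancing one step per activation.
; Each step locks movement, plays cast montages and, after a delay, shoots a projectile forward with damage scaled from the user's AttackPower stat.
; The first two steps start a timer that resets the combo.
; The third uses its own fireball class and sound, then resets the count and starts the ability cooldown.
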(event `self.OnActivateAbility`
  (bind _returnvalue (`StatContainer.GetStat` (`self.StatContainer`) "AttackPower"))
  (`/Engine/EditorBlueprintResources/StandardMacros.IsValid` _returnvalue
    (:`Is Valid`
      (set `self.attackPower` (`Stat.GetValue` _returnvalue))
      (`self.SetPlayerFreeStat` false)
      (switch `int` (`self.CurrentProjectileCount`)
        (:`0`
          ;[1 1 1] First Fireball
          (`Character.PlayAnimMontage` (`self.CurrentUser`) "/Game/Blueprints/Animations/Character/Montages/AM_FireArcana1_P1.AM_FireArcana1_P1" 1.0 "None")
          (`self.MakeFireBall` (`self.DamgeMulti_1`) (`self.CastTime_1`) (`self.FireBallActor`) "/Game/Sounds/fire_1.fire_1")
          (set `self.CurrentProjectileCount` (+ (`self.CurrentProjectileCount`) 1))
          (bind _returnvalue_2 (`Character.PlayAnimMontage` (`self.CurrentUser`) "/Game/Blueprints/Animations/Character/Montages/AM_FireArcana1_P2.AM_FireArcana1_P2" 1.0 "None"))
          (`KismetSystemLibrary.Delay` _returnvalue_2)
          (`self.StartRecetCycleCooldown`))
        (:`1`
          ;[1 1 1] Second Fireball
          (`Character.PlayAnimMontage` (`self.CurrentUser`) "/Game/Blueprints/Animations/Character/Montages/AM_FireArcana2_P1.AM_FireArcana2_P1" 1.0 "None")
          (`self.MakeFireBall` (`self.DamgeMulti_2`) (`self.CastTime_2`) (`self.FireBallActor`) "/Game/Sounds/fire_1.fire_1")
          (set `self.CurrentProjectileCount` (+ (`self.CurrentProjectileCount`) 1))
          (bind _returnvalue_3 (`Character.PlayAnimMontage` (`self.CurrentUser`) "/Game/Blueprints/Animations/Character/Montages/AM_FireArcana2_P2.AM_FireArcana2_P2" 1.0 "None"))
          (`KismetSystemLibrary.Delay` _returnvalue_3)
          (`self.StartRecetCycleCooldown`))
        (:`2`
          ;[1 1 1] Third FireBall
          (`Character.PlayAnimMontage` (`self.CurrentUser`) "/Game/Blueprints/Animations/Character/Montages/AM_FireArcana3_P1.AM_FireArcana3_P1" 1.0 "None")
          (`self.MakeFireBall` (`self.DamgeMulti_3`) (`self.CastTime_3`) (`self.ThirdFireBallActor`) "/Game/Sounds/fire_2_impact.fire_2_impact")
          (set `self.CurrentProjectileCount` 0)
          (`self.StartCooldown`)
          (bind _returnvalue_4 (`Character.PlayAnimMontage` (`self.CurrentUser`) "/Game/Blueprints/Animations/Character/Montages/AM_FireArcana3_P2.AM_FireArcana3_P2" 1.0 "None"))
          (`KismetSystemLibrary.Delay` _returnvalue_4)))
      (`self.SetPlayerFreeStat` true))
    (:`Is Not Valid`
      (`KismetSystemLibrary.PrintString` "FireArcana: Not Ayyack power stat found" false))))

(event `OnRecetCycle`
  (set `self.CurrentProjectileCount` 0))

(fn `MultiAttackPower`
  (params (Multi :type "Float (double-precision)"))
  (set `self.attackPower` (* Multi (`self.attackPower`))))

(fn `SetPlayerFreeStat`
  (params (State :type Boolean))
  (set `PlayerCharacter.CanMove` State (`self.CurrentUser`)))

(fn `SpawnFireBall`
  (params (fireBall :type "FireballArcanaProjectile Class Reference"))
  (locals (direction :type "Vector Structure"))
  (bind _currentuser (`self.CurrentUser`))
  (set `local.direction` (`self.GetActorForwardVector` _currentuser))
  (bind _returnvalue (`|SpawnActorFromClass` fireBall (`KismetMathLibrary.MakeTransform` (+ (`self.K2_GetActorLocation` _currentuser) (* (`local.direction`) (`self.FireBallSpawnDistance`))) (`self.K2_GetActorRotation` (`self.CurrentUser`))) "Undefined" "MultiplyWithRoot" null null))
  (`FireballArcanaProjectile.Shoot` _returnvalue null (`self.FireBallSpeed`) (`local.direction`) (`self.attackPower`)))

(fn `UserConstructionScript`)