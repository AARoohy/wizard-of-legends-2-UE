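; BP_PlayerCharacter is the player character, with stat-driven movement, a dash and one ability slot.
; BeginPlay seeds base stats in StatContainer, caches the move-speed and health stats, pulls the slot ability from AbilityDataBase and creates the gameplay HUD.
; Movement is camera-relative with interpolated rotation, while dash launches along the input direction on a cooldown.
; Gate macros block all three actions when dead; movement and the ability also require CanMove.
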(event `self.ReceiveBeginPlay`
  (`|ExecutionSequence`
    (:`then_0`
      ;[1 1 1] Set Stats Base values
      (`StatContainer.AddModifier` (`self.StatContainer`) (make `StatModifier` "Health" "Base" 100.0))
      (`StatContainer.AddModifier` (`self.StatContainer`) (make `StatModifier` "MoveSpeed" "Base" 1000.0))
      (`StatContainer.AddModifier` (`self.StatContainer`) (make `StatModifier` "AttackPower" "Base" 15.0)))
    (:`then_1`
      ;[1 1 1] Get Stats
      (bind _returnvalue (`StatContainer.GetStat` (`self.StatContainer`) "MoveSpeed"))
      (bind _asmove_speed_stat (cast `MoveSpeedStat` _returnvalue))
      (set `self.moveSpeedStat` _asmove_speed_stat)
      (bind _returnvalue_2 (`StatContainer.GetStat` (`self.StatContainer`) "Health"))
      (bind _ashealth_stat (cast `HealthStat` _returnvalue_2))
      (set `self.HealthStat` _ashealth_stat))
    (:`then_2`
      ;[1 1 1] Set Ability First Slot
      (set `self.AbilitySlot1` (`AbilityDatabase.GetAbilityInstanceByID` (`self.AbilityDataBase`) 1 self)))
    (:`then_3`
      ;[1 1 1] Setup Player HUD
      (bind _returnvalue_3 (`|CreateWidget` "/Game/Widgets/GamePlay/WB_Gameplay_HUD.WB_Gameplay_HUD_C" (`GameplayStatics.GetPlayerController` 0)))
      (`UserWidget.AddToViewport` _returnvalue_3 0)
      (`/Game/Widgets/GamePlay/WB_Gameplay_HUD.Setup` _returnvalue_3 self))))

(event `self.ReceiveTick`
  (params (DeltaSeconds :type "Float (single-precision)"))
  (set `self.deltaTime` DeltaSeconds))

(event `EnhancedInput|/Game/Input/Actions/IA_Move`
  (params (ActionValue :type "Vector2D Structure") (ElapsedSeconds :type "Float (double-precision)") (TriggeredSeconds :type "Float (double-precision)") (InputAction :type "InputAction Object Reference" :default "/Game/Input/Actions/IA_Move.IA_Move"))
  ;[1 1 1] Movement
  (:`Triggered`
    (`self.Is Not Dead`
      (:`Output`
        (`self.Is Free`
          (:`Output`
            (set `self.inputDirection` (`KismetMathLibrary.MakeVector` ActionValue_Y ActionValue_X))
            (bind _returnvalue (`self.DirectionBasedOnCamera` (`self.inputDirection`) (`self.Camera`)))
            (bind _output_get (set `self.inputDirection` _returnvalue))
            (`self.AddMovementInput` (`KismetMathLibrary.MakeVector` (.x _output_get) (.y _output_get)) (* (`self.deltaTime`) (`Stat.GetValue` (`self.moveSpeedStat`))))
            (`self.K2_SetActorRotation` (`KismetMathLibrary.RInterpTo` (`self.K2_GetActorRotation`) (`KismetMathLibrary.MakeRotFromX` (`self.inputDirection`)) (`self.deltaTime`) 5.0)))))))
  (:`Canceled`
    (set `self.inputDirection` (0.0 0.0 0.0) :!label _label))
  (:`Completed`
    (goto _label)))

(event `EnhancedInput|/Game/Input/Actions/IA_Dash`
  (params (ActionValue :type Boolean) (ElapsedSeconds :type "Float (double-precision)") (TriggeredSeconds :type "Float (double-precision)") (InputAction :type "InputAction Object Reference" :default "/Game/Input/Actions/IA_Dash.IA_Dash"))
  ;[1 1 1] Dash
  (:`Started`
    (`self.Is Not Dead`
      (:`Output`
        (if (> (`KismetMathLibrary.VSize` (`self.inputDirection`)) 0.0)
          (if (`self.canDash`)
            (`self.LaunchCharacter` (* (`self.inputDirection`) (`self.dashPower`)))
            (set `self.canDash` false)
            (`KismetSystemLibrary.Delay` (`self.dashCooldown`))
            (set `self.canDash` true)))))))

(event `EnhancedInput|/Game/Input/Actions/IA_FirstSlot`
  (params (ActionValue :type Boolean) (ElapsedSeconds :type "Float (double-precision)") (TriggeredSeconds :type "Float (double-precision)") (InputAction :type "InputAction Object Reference" :default "/Game/Input/Actions/IA_FirstSlot.IA_FirstSlot"))
  ;[1 1 1] Activate First Slot Ability
  (:`Started`
    (`self.Is Not Dead`
      (:`Output`
        (`self.Is Free`
          (:`Output`
            (`BaseAbility.ActivateAbility` (`self.AbilitySlot1`) self)))))))

(event `Key|Enter`
  (params (Key :type "Key Structure"))
  (:`Pressed`
    (`KismetSystemLibrary.PrintString` (`KismetStringLibrary.Conv_BoolToString` (`HealthStat.GetIsDead` (`self.HealthStat`))))))

(fn `UserConstructionScript`)