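; BP_Dummy is a damageable enemy dummy with stat-driven health and an on-actor HUD.
; On BeginPlay it caches its HealthStat from the StatContainer, applies base stat modifiers, sets up the HUD and binds to death.
; Damage reveals the HUD, records the damager, lowers health, spawns a damage popup while alive and plays a random hit montage.
; Death reports the killer through the game instance, plays a sound and destroys the actor.
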(event `self.ReceiveBeginPlay`
  (`|ExecutionSequence`
    (:`then_0`
      (bind _returnvalue (`StatContainer.GetStat` (`self.StatContainer`) "Health"))
      (bind _ashealth_stat (cast `HealthStat` _returnvalue))
      (set `self.Health Stat` _ashealth_stat))
    (:`then_1`
      (for _array_element (`self.BaseStats`)
        (`StatContainer.AddModifier` (`self.StatContainer`) _array_element)))
    (:`then_2`
      (bind _aswb_enemy_hud (cast `/Game/Widgets/GamePlay/WB_EnemyHUD` (`WidgetComponent.GetWidget` (`self.HUD`))))
      (`/Game/Widgets/GamePlay/WB_EnemyHUD.Setup` _aswb_enemy_hud (`self.Health Stat`)))
    (:`then_3`
      (add `HealthStat.OnDied` (`self.Health Stat`) (`|CreateDelegate` :!event `OnCharacterDie`)))))

(event `self.ReceiveAnyDamage`
  (params (Damage :type "Float (single-precision)") (DamageType :type "DamageType Object Reference") (InstigatedBy :type "Controller Object Reference") (DamageCauser :type "Actor Object Reference"))
  (`|ExecutionSequence`
    (:`then_0`
      (if (not (`SceneComponent.IsVisible` (`self.HUD`)))
        (`SceneComponent.SetVisibility` (`self.HUD`) true false)))
    (:`then_1`
      (set `self.LastDamager` DamageCauser))
    (:`then_2`
      (`HealthStat.DecreaseCurrentHealth` (`self.Health Stat`) Damage))
    (:`then_3`
      (if (not (`HealthStat.GetIsDead` (`self.Health Stat`)))
        (`/Game/Blueprints/Macros/PopupMacro.PopupTextSpawn` "/Game/Blueprints/PopupText/Blueprints/BP_DamagePopup.BP_DamagePopup_C" (`SceneComponent.K2_GetComponentLocation` (`self.Arrow`)) (`KismetTextLibrary.Conv_DoubleToText` Damage "HalfToEven"))))
    (:`then_4`
      (`|PlayMontage` (`self.SK_Dummy`) (select `int` (`KismetMathLibrary.RandomInteger` 2) :`0` "/Game/Blueprints/Animations/Dummy/AM_DummyHit1.AM_DummyHit1" :`1` "/Game/Blueprints/Animations/Dummy/AM_DummyHit2.AM_DummyHit2" :!type "AnimMontage Object Reference")))))

(fn `OnCharacterDie`
  (bind _asgib_game_instance (cast `/Game/Blueprints/GIB_GameInstance` (`GameplayStatics.GetGameInstance`)))
  (`/Game/Blueprints/GIB_GameInstance.OnEnemyDied` _asgib_game_instance (make `/Game/Structures/S_DummyDeathEventData` (`self.LastDamager`) self))
  (`GameplayStatics.PlaySound2D` "/Game/Sounds/enemy_dead.enemy_dead" 1.0 1.0 0.0 null null)
  (`self.K2_DestroyActor`))

(fn `UserConstructionScript`)