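; Player character Blueprint handling camera-relative movement, a dash, a first-slot ability and kill-streak tracking.
; BeginPlay seeds StatContainer base modifiers, caches stats, creates the slot ability from a database, builds the HUD and binds enemy deaths to the streak.
; Input passes alive and free checks; dash overrides velocity, with CanDash blocking movement and re-dashing until its delay ends.
; The V key simulates taking random damage.
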(event `self.ReceiveTick`
  (params (DeltaSeconds :type "Float (single-precision)"))
  (set `self.deltaTime` DeltaSeconds))

(event `EnhancedInput|/Game/Input/Actions/IA_Move`
  (params (ActionValue :type "Vector2D Structure") (ElapsedSeconds :type "Float (double-precision)") (TriggeredSeconds :type "Float (double-precision)") (InputAction :type "InputAction Object Reference" :default "/Game/Input/Actions/IA_Move.IA_Move"))
  ;[1 1 1] Movement
  (:`Triggered`
    (`self.Is Not Dead`
      (:`Output`
        (`self.Is Free`
          (:`Output`
            (if (`self.canDash`)
              (set `self.inputDirection` (`KismetMathLibrary.MakeVector` ActionValue_Y ActionValue_X))
              (bind _returnvalue (`self.DirectionBasedOnCamera` (`self.inputDirection`) (`self.Camera`)))
              (bind _output_get (set `self.inputDirection` _returnvalue))
              (`self.AddMovementInput` (`KismetMathLibrary.MakeVector` (.x _output_get) (.y _output_get)) (* (`self.deltaTime`) (`Stat.GetValue` (`self.moveSpeedStat`))))
              (`self.K2_SetActorRotation` (`KismetMathLibrary.RInterpTo` (`self.K2_GetActorRotation`) (`KismetMathLibrary.MakeRotFromX` (`self.inputDirection`)) (`self.deltaTime`) 5.0))))))))
  (:`Canceled`
    (set `self.inputDirection` (0.0 0.0 0.0) :!label _label))
  (:`Completed`
    (goto _label)))

(event `self.ReceiveBeginPlay`
  (set `self.CanMove` true)
  (`|ExecutionSequence`
    (:`then_0`
      ;[1 1 1] Set Stats Base values
      (`StatContainer.AddModifier` (`self.StatContainer`) (make `StatModifier` "Health" "Base" 100.0))
      (`StatContainer.AddModifier` (`self.StatContainer`) (make `StatModifier` "MoveSpeed" "Base" 1000.0))
      (`StatContainer.AddModifier` (`self.StatContainer`) (make `StatModifier` "AttackPower" "Base" 15.0)))
    (:`then_1`
      ;[1 1 1] Get Stats
      (bind _returnvalue (`StatContainer.GetStat` (`self.StatContainer`) "MoveSpeed"))
      (bind _asmove_speed_stat (cast `MoveSpeedStat` _returnvalue))
      (set `self.moveSpeedStat` _asmove_speed_stat)
      (bind _returnvalue_2 (`StatContainer.GetStat` (`self.StatContainer`) "Health"))
      (bind _ashealth_stat (cast `HealthStat` _returnvalue_2))
      (set `self.HealthStat` _ashealth_stat))
    (:`then_2`
      ;[1 1 1] Set Ability First Slot
      (bind _output_get (set `self.AbilitySlot1` (`AbilityDatabase.GetAbilityInstanceByID` (`self.AbilityDataBase`) 1 self)))
      (`BaseAbility.Setup` _output_get self))
    (:`then_3`
      ;[1 1 1] Setup Player HUD
      (bind _returnvalue_3 (`|CreateWidget` "/Game/Widgets/GamePlay/WB_Gameplay_HUD.WB_Gameplay_HUD_C" (`GameplayStatics.GetPlayerController` 0)))
      (`UserWidget.AddToViewport` _returnvalue_3 0)
      (`/Game/Widgets/GamePlay/WB_Gameplay_HUD.Setup` _returnvalue_3 self))
    (:`then_4`
      ;[1 1 1] Bind to EnemyDeath
      (bind _asgib_game_instance (cast `/Game/Blueprints/GIB_GameInstance` (`GameplayStatics.GetGameInstance`)))
      (add `/Game/Blueprints/GIB_GameInstance.OnEnemyDied` _asgib_game_instance (delegate `OnDummyDied_Event`)))))

(event `EnhancedInput|/Game/Input/Actions/IA_Dash`
  (params (ActionValue :type Boolean) (ElapsedSeconds :type "Float (double-precision)") (TriggeredSeconds :type "Float (double-precision)") (InputAction :type "InputAction Object Reference" :default "/Game/Input/Actions/IA_Dash.IA_Dash"))
  ;[1 1 1] Dash
  (:`Started`
    (`self.Is Not Dead`
      (:`Output`
        (`self.Is Free`
          (:`Output`
            (if (> (`KismetMathLibrary.VSize` (`self.inputDirection`)) 0.0)
              (if (`self.canDash`)
                (`self.K2_SetActorRotation` (`KismetMathLibrary.MakeRotFromX` (`self.inputDirection`)))
                (set `MovementComponent.Velocity` (* (`self.inputDirection`) (`self.dashPower`)) (`self.CharacterMovement`))
                (set `self.canDash` false)
                (`GameplayStatics.SpawnEmitterAttached` "/Game/Plugins/FXVarietyPack/Particles/P_ky_shotShockwave.P_ky_shotShockwave" (`self.Mesh`) "None" (`self.K2_GetActorLocation` self) (`self.K2_GetActorRotation` self) (1.0 1.0 1.0) "KeepWorldPosition")
                (`GameplayStatics.PlaySound2D` "/Game/Sounds/dash.dash" 1.0 1.0 0.0 null null)
                (`KismetSystemLibrary.Delay` (`self.dashDuration`))
                (set `self.canDash` true)
                (set `MovementComponent.Velocity` (* (`self.inputDirection`) (`Stat.GetValue` (`self.moveSpeedStat`))) (`self.CharacterMovement`))))))))))

(event `OnDummyDied_Event`
  (params (Event :type "/Game/Structures/S_DummyDeathEventData Structure"))
  ;[1 1 1] Bind to EnemyDeath
  (if (== Event_Killer_3_EA82591D4DAC1C3E1A7C1894165A06D8 self)
    (`self.AddKillStreak` 1)))

(event `EnhancedInput|/Game/Input/Actions/IA_FirstSlot`
  (params (ActionValue :type Boolean) (ElapsedSeconds :type "Float (double-precision)") (TriggeredSeconds :type "Float (double-precision)") (InputAction :type "InputAction Object Reference" :default "/Game/Input/Actions/IA_FirstSlot.IA_FirstSlot"))
  ;[1 1 1] Activate First Slot Ability
  (:`Started`
    (`self.Is Not Dead`
      (:`Output`
        (`self.Is Free`
          (:`Output`
            (`BaseAbility.ActivateAbility` (`self.AbilitySlot1`))))))))

(event `Key|V`
  (params (Key :type "Key Structure"))
  ;[1 1 1] Hit Simulation
  (:`Pressed`
    (`HealthStat.DecreaseCurrentHealth` (`self.HealthStat`) (`KismetMathLibrary.Conv_IntToDouble` (`KismetMathLibrary.Round` (`KismetMathLibrary.RandomFloatInRange` 7.0 15.0))))))

(fn `AddKillStreak`
  (params (amount :type Integer))
  (locals (oldValue :type Integer))
  (bind _killstreak (`self.KillStreak`))
  (bind _output_get (set `local.oldValue` _killstreak))
  (bind _output_get_2 (set `self.KillStreak` (+ _killstreak amount)))
  (`self.OnKillStreakChanged` _output_get _output_get_2))

(fn `UserConstructionScript`)