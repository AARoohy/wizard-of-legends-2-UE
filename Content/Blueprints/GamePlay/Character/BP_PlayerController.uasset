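; BP_PlayerController is a player controller that configures input and mouse behavior when play begins.
; BeginPlay calls Set Game Mode Only and adds the IMC_Default Enhanced Input mapping context at elevated priority.
; Set Game Mode Only applies game-only input and permanent viewport mouse capture while keeping the cursor visible, including during capture.
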(event `self.ReceiveBeginPlay`
  (`WidgetBlueprintLibrary.SetInputMode_GameOnly` self true)
  (`GameplayStatics.SetViewportMouseCaptureMode` "CapturePermanently_IncludingInitialMouseDown")
  (set `PlayerController.bShowMouseCursor` true)
  (`self.SetHideCursorDuringCapture` false)
  (`EnhancedInputSubsystemInterface.AddMappingContext` (pcsubsystem `EnhancedInputLocalPlayerSubsystem` self) "/Game/Input/IMC_Default.IMC_Default" 10 (struct)))

(fn `UserConstructionScript`)