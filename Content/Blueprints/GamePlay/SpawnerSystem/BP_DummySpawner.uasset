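; BP_DummySpawner is a spawner that places actors of a configurable dummy class at predefined positions.
; BeginPlay starts a looping timer at the spawn cooldown, while CheckForSpawn uses a GetFreePos macro to find the first position that is not full.
; Spawn creates the actor at that position's transform and registers it there through SetObject, with debug prints along the way.
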(event `self.ReceiveBeginPlay`
  (`KismetSystemLibrary.K2_SetTimerDelegate` (`|CreateDelegate` :!event `CheckForSpawn`) (`self.SpawnCooldown`) true))

(fn `CheckForSpawn`
  (bind _spawnpos (`self.GetFreePos`)
    (:`Output`
      (`KismetSystemLibrary.PrintString` "part 2")
      (`self.Spawn` _spawnpos))))

(fn `Spawn`
  (params (SpawnPos :type "/Game/Blueprints/GamePlay/SpawnerSystem/BP_SpawnPos Object Reference"))
  (bind _returnvalue (`|SpawnActorFromClass` (`self.DummyClass`) (`self.GetTransform` SpawnPos) "Undefined" "MultiplyWithRoot" null null))
  (`/Game/Blueprints/GamePlay/SpawnerSystem/BP_SpawnPos.SetObject` SpawnPos _returnvalue)
  (`KismetSystemLibrary.PrintString` "Hello"))

(fn `UserConstructionScript`)